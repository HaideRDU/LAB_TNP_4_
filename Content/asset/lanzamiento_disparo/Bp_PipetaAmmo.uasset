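; Pipette ammo projectile whose initial speed comes from its Impulso variable, set in the construction script.
; On sphere overlap with scenery, a Caldera, a Caldera spawner or an Enemy, it spawns the AGUA_disparo effect at the Diparo component and destroys itself.
; Hitting an Enemy first calls SeguirAumentandoTamano on it to keep increasing its size; overlaps with any other actor are ignored.
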(event `self.Sphere.OnComponentBeginOverlap`
  (params (OverlappedComponent :type "PrimitiveComponent Object Reference") (OtherActor :type "Actor Object Reference") (OtherComp :type "PrimitiveComponent Object Reference") (OtherBodyIndex :type Integer) (bFromSweep :type Boolean) (SweepResult :type "HitResult Structure (by ref)"))
  (cast `/Game/asset/map/props/ESCENARIO/bp_escenario` OtherActor
    (:`then`
      _)
    (:`CastFailed`
      (cast `/Game/asset/map/props/Bp_Caldera` OtherActor
        (:`then`
          _)
        (:`CastFailed`
          (cast `/Game/asset/map/props/Bp_Caldera_Spawer` OtherActor
            (:`then`
              _)
            (:`CastFailed`
              (bind _asenemy (cast `/Game/Characters/ENEMY/Enemy` OtherActor))
              (`/Game/Characters/ENEMY/Enemy.seguir aumentando tamano` _asenemy)))))))
  (`NiagaraFunctionLibrary.SpawnSystemAtLocation` "/Game/Characters/ENEMY/AGUA_disparo.AGUA_disparo" (`SceneComponent.GetSocketLocation` (`self.diparo`) "None"))
  (`self.K2_DestroyActor`))

(fn `UserConstructionScript`
  (set `ProjectileMovementComponent.InitialSpeed` (`self. Impulso`) (`self.ProjectileMovement`)))