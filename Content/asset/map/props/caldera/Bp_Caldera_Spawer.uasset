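; Cauldron prop ("Caldera") Blueprint that acts as an enemy spawner, keeping one AI enemy alive at a time.
; A looping timer started on BeginPlay periodically prunes invalid entries from the tracked enemy array, then triggers the spawn check.
; When the array is empty, it spawns an AI pawn at a random point within the cylinder component's bounds and records it.
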(event `self.ReceiveBeginPlay`
  (`KismetSystemLibrary.K2_SetTimerDelegate` (delegate `revisar_enemigos`) 5.0 true))

(event `revisar_enemigos`
  (bind (_arrayindex _arrayelement) (`/Engine/EditorBlueprintResources/StandardMacros.ReverseForEachLoop` (`self.Enemy`))
    (:`LoopBody`
      (`/Engine/EditorBlueprintResources/StandardMacros.IsValid` _arrayelement
        (:`Is Not Valid`
          (`KismetArrayLibrary.Array_Remove` (`self.Enemy`) _arrayindex))))
    (:`Completed`
      (`self.Spawn_enemigos`))))

(event `Spawn_enemigos`
  (bind _returnvalue (`KismetArrayLibrary.Array_Length` (`self.Enemy`)))
  (bind (_origin _boxextent) (`KismetSystemLibrary.GetComponentBounds` (`self.caldera_cilindro`)))
  (if (< _returnvalue 1)
    (for _ (range 1 (+ (- 1 _returnvalue) 1))
      (bind _returnvalue_2 (`AIBlueprintHelperLibrary.SpawnAIFromClass` "/Game/Characters/ENEMY/Enemy.Enemy_C" null (`KismetMathLibrary.RandomPointInBoundingBox` _origin _boxextent) (struct) false null))
      (`KismetArrayLibrary.Array_Add` (`self.Enemy`) _returnvalue_2))))

(fn `UserConstructionScript`)